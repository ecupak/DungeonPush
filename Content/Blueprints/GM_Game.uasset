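; Game mode that builds the level from streamed chunks laid out along the X axis and starts play.
; LoadChunk spawns a soft-referenced level instance at the next location, then advances it by LevelGap.
; Only the newest and previous chunks are tracked, and UnloadChunk requests removal of the previous one.
; BeginPlay loads the first chunk and, shortly after it finishes loading, calls StartLevel on BP_PlayerPawn.
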(event `self.ReceiveBeginPlay`
  (`self.LoadChunk` "/Game/Levels/Level_Chunk_00.Level_Chunk_00")
  (add `LevelStreaming.OnLevelLoaded` (`self.NewChunk`) (`|CreateDelegate` :!event `Bind_OnLevelLoaded`)))

(event `Bind_OnLevelLoaded`
  (`KismetSystemLibrary.Delay` 0.2)
  (bind _returnvalue (`GameplayStatics.GetActorOfClass` "/Game/Blueprints/TrackItems/Player/BP_PlayerPawn.BP_PlayerPawn_C"))
  (`/Game/Blueprints/TrackItems/Player/BP_PlayerPawn.StartLevel` _returnvalue))

(event `LoadChunk`
  (params (Level :type "World Soft Object Reference"))
  (bind (_boutsuccess _returnvalue) (`LevelStreamingDynamic.LoadLevelInstanceBySoftObjectPtr` Level (`self.NextLevelLocation`) (struct) "" null))
  (`self.StoreNewestChunk` _returnvalue)
  (`self.CalculateNextLevelLocation`))

(event `UnloadChunk`
  (bind _oldchunk (`self.OldChunk`)
    (:`then`
      (`LevelStreaming.SetIsRequestingUnloadAndRemoval` _oldchunk true))
    (:`else`)))

(fn `CalculateNextLevelLocation`
  (bind (_nextlevellocation_x _nextlevellocation_y _nextlevellocation_z) (`KismetMathLibrary.BreakVector` (`self.NextLevelLocation`)))
  (set `self.NextLevelLocation` (`KismetMathLibrary.MakeVector` (+ _nextlevellocation_x (`self.LevelGap`)) _nextlevellocation_y _nextlevellocation_z))
  (return))

(fn `StoreNewestChunk`
  (params (NewestChunk :type "LevelStreamingDynamic Object Reference"))
  (set `self.OldChunk` (`self.NewChunk`))
  (set `self.NewChunk` (`local.NewestChunk`))
  (return))

(fn `UserConstructionScript`)