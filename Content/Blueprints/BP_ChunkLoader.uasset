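; BP_ChunkLoader is a trigger actor that streams a level chunk in and out as the player passes through its LevelTrigger volume.
; The first overlap by BP_PlayerPawn asks GM_Game to load the chunk named by its Level variable.
; The first exit calls UnloadChunk on the game mode without specifying a level.
; Separate DoOnce gates keep each action from repeating.
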(event `self.LevelTrigger.OnComponentBeginOverlap`
  (params (OverlappedComponent :type "PrimitiveComponent Object Reference") (OtherActor :type "Actor Object Reference") (OtherComp :type "PrimitiveComponent Object Reference") (OtherBodyIndex :type Integer) (bFromSweep :type Boolean) (SweepResult :type "HitResult Structure (by ref)"))
  (cast `/Game/Blueprints/TrackItems/Player/BP_PlayerPawn` OtherActor) ; Only do this when the player touches it,\nand only do it once.
  (`/Engine/EditorBlueprintResources/StandardMacros.DoOnce` false
    (:`Completed`
      (`/Game/Blueprints/GM_Game.LoadChunk` (cast `/Game/Blueprints/GM_Game` (`GameplayStatics.GetGameMode`) :!pure true) (`self.Level`)))))

(event `self.LevelTrigger.OnComponentEndOverlap`
  (params (OverlappedComponent :type "PrimitiveComponent Object Reference") (OtherActor :type "Actor Object Reference") (OtherComp :type "PrimitiveComponent Object Reference") (OtherBodyIndex :type Integer))
  (cast `/Game/Blueprints/TrackItems/Player/BP_PlayerPawn` OtherActor) ; Only do this when the player leaves it,\nand only do it once.
  (`/Engine/EditorBlueprintResources/StandardMacros.DoOnce` false
    (:`Completed`
      (`/Game/Blueprints/GM_Game.UnloadChunk` (cast `/Game/Blueprints/GM_Game` (`GameplayStatics.GetGameMode`) :!pure true)))))

(fn `UserConstructionScript`)