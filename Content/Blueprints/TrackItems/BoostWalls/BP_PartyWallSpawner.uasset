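; BP_PartyWallSpawner is a track item that periodically spawns BP_PartyWall actors, alternating between left and right arrow positions.
; Looping timers set up on BeginPlay govern spawning and difficulty.
; Each wall takes the spawner's rotation and is initialized with the current wall value and movement speed.
; Difficulty increases multiply the wall value for subsequent spawns and print the new value.
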(event `self.ReceiveBeginPlay`
  (`KismetSystemLibrary.K2_SetTimerDelegate` (`|CreateDelegate` :!event `SpawnWall`) (`self.SpawnDelay`) true)
  (`KismetSystemLibrary.K2_SetTimerDelegate` (`|CreateDelegate` :!event `IncreaseDifficulty`) (`self.DifficultyDelay`) true))

(event `SpawnWall`
  (bind _spawnlocation (`self.GetSpawnLocation`))
  (bind _returnvalue (`|SpawnActorFromClass` "/Game/Blueprints/TrackItems/BoostWalls/BP_PartyWall.BP_PartyWall_C" (`KismetMathLibrary.MakeTransform` _spawnlocation (`self.K2_GetActorRotation`)) "AlwaysSpawn" "MultiplyWithRoot" null null))
  (`/Game/Blueprints/TrackItems/BoostWalls/BP_PartyWall.Initialize` _returnvalue (`self.WallValue`) (`self.MovementSpeed`)))

(event `IncreaseDifficulty`
  (bind _output_get (set `self.WallValue` (* (`self.WallValue`) 1.5)))
  (`KismetSystemLibrary.PrintText` (`|FormatText` "Wall value is now {x}" _output_get)))

(fn `GetSpawnLocation`
  (returns (SpawnLocation :type "Vector Structure"))
  (bind _output_get (set `self.IsLeftSide` (not (`self.IsLeftSide`))))
  (if _output_get
    (return (`SceneComponent.K2_GetComponentLocation` (`self.ArrowLeft`)))
    (else
      (return (`SceneComponent.K2_GetComponentLocation` (`self.ArrowRight`))))))

(fn `UserConstructionScript`)