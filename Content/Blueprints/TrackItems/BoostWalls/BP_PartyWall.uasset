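; BP_PartyWall is a boost-wall track item whose displayed value rises by the damage of each shot it takes.
; Initialize sets the starting value and movement speed, and the Shot event adds damage to that value.
; Both push the floored value to a WBP_PartyWall widget, cached from the widget component on BeginPlay.
; GetHeight returns the full height of the wall's scaled box.
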(event `self.ReceiveBeginPlay`
  (`parent.ReceiveBeginPlay`)
  (bind _aswbp_party_wall (cast `/Game/Widgets/WBP_PartyWall` (`WidgetComponent.GetWidget` (`self.Widget`))))
  (set `self.PartyWallWidget` _aswbp_party_wall))

(event `/Game/Blueprints/Bullet/BPI_Shootable.ReceiveShot`
  (params (Damage :type "Float (double-precision)"))
  (bind _output_get (set `self.Value` (+ Damage (`self.Value`))))
  (`/Game/Widgets/WBP_PartyWall.SetValue` (`self.PartyWallWidget`) (`KismetMathLibrary.FFloor` _output_get)))

(fn `GetHeight`
  (returns (Height :type "Float (double-precision)"))
  (bind (_returnvalue_x _returnvalue_y _returnvalue_z) (`KismetMathLibrary.BreakVector` (`BoxComponent.GetScaledBoxExtent` (`self.Box`))))
  (return (* _returnvalue_z 2.0)))

(fn `Initialize`
  (params (InitValue :type "Float (double-precision)") (InitSpeed :type "Float (double-precision)"))
  (`|ExecutionSequence`
    (:`then_0`
      (bind _output_get (set `self.Value` (`local.InitValue`)))
      (`/Game/Widgets/WBP_PartyWall.SetValue` (`self.PartyWallWidget`) (`KismetMathLibrary.FFloor` _output_get)))
    (:`then_1`
      (set `self.MovementSpeed` (`local.InitSpeed`)))))

(fn `UserConstructionScript`)