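; Base track item pawn that is placed on a track and then moves forward along its facing direction.
; On BeginPlay, the ACPlaceOnTrack component positions it using GetHeight, which returns zero here.
; Every tick, MoveTowardsEnd feeds the forward vector scaled by MovementSpeed into AddMovementInput.
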(event `self.ReceiveBeginPlay`
  (`/Game/Blueprints/TrackItems/AC_PlaceOnTrack.PlaceOnTrack` (`self.AC_PlaceOnTrack`) self (`self.GetHeight`)))

(event `self.ReceiveTick`
  (params (DeltaSeconds :type "Float (single-precision)"))
  (`self.MoveTowardsEnd`))

(fn `GetHeight`
  (returns (Height :type "Float (double-precision)"))
  (return 0.0))

(fn `MoveTowardsEnd`
  (`self.AddMovementInput` (* (`self.GetActorForwardVector`) (`self.MovementSpeed`)))
  (return))

(fn `UserConstructionScript`)