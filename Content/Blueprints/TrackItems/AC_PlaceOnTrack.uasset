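; AC_PlaceOnTrack is an actor component that snaps a given actor onto the surface beneath it, used for track items.
; PlaceOnTrack traces on the Visibility channel along the actor's local down vector, so placement follows the actor's orientation rather than world down.
; On a hit it teleports the actor to half the given height above the impact along its up vector; otherwise it prints a warning.
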(event `PlaceOnTrack`
  (params (ActorToPlace :type "Actor Object Reference") (Height :type "Float (double-precision)"))
  (bind (_wasgroundfound _groundlocation) (`self.FindGround` ActorToPlace))
  (if _wasgroundfound
    (`self.PlaceActorOnGround` ActorToPlace _groundlocation Height)
    (else
      (`KismetSystemLibrary.PrintString` "No ground"))))

(fn `FindGround`
  (params (ActorToPlace :type "Actor Object Reference"))
  (returns (WasGroundFound :type Boolean) (GroundLocation :type "Vector Structure"))
  (bind _returnvalue (`Actor.K2_GetActorLocation` ActorToPlace))
  (bind (_outhit _returnvalue_2) (`KismetSystemLibrary.LineTraceSingle` _returnvalue (+ _returnvalue (* (`Actor.GetActorUpVector` (`local.ActorToPlace`)) -1000.0)) "TraceTypeQuery1" false (`|MakeArray` (`local.ActorToPlace`) null) "ForOneFrame" true (struct :`R` 1.0 :`A` 1.0) (struct :`G` 1.0 :`A` 1.0) 1.0))
  (return _returnvalue_2 (`.Location` (`GameplayStatics.BreakHitResult` _outhit))))

(fn `PlaceActorOnGround`
  (params (ActorToPlace :type "Actor Object Reference") (GroundLocation :type "Vector Structure") (Height :type "Float (double-precision)"))
  (`Actor.K2_SetActorLocation` ActorToPlace (+ GroundLocation (* Height (`Actor.GetActorUpVector` (`local.ActorToPlace`)) 0.5)) false true)
  (return))