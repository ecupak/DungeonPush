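; Player squad component that manages a row of BP_Unit actors attached to a box component passed in through Initialize.
; AddUnit spawns and attaches a unit, while RemoveUnit destroys the last one, each printing a debug message.
; Each successful change triggers RealignSquad, which scales the box's Y extent with unit count and spaces units evenly along local Y, centered on the box.
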(event `Initialize`
  (params (SquadBox :type "BoxComponent Object Reference"))
  (set `self.Squad Box` SquadBox))

(event `AddUnit`
  (bind _returnvalue (`|SpawnActorFromClass` "/Game/Blueprints/TrackItems/Player/BP_Unit.BP_Unit_C" (`KismetMathLibrary.MakeTransform` (0.0 0.0 0.0)) "Undefined" "MultiplyWithRoot" null null))
  (`KismetArrayLibrary.Array_Add` (`self.All_Unit`) _returnvalue)
  (`Actor.K2_AttachToComponent` _returnvalue (`self.Squad Box`) "None" "KeepRelative" "KeepRelative" "KeepRelative" false)
  (`KismetSystemLibrary.PrintString` "Added")
  (`self.RealignSquad`))

(event `RemoveUnit`
  (bind _all_unit (`self.All_Unit`))
  (bind _returnvalue (`KismetArrayLibrary.Array_LastIndex` _all_unit))
  (bind _output (`|GetArrayItem` _all_unit _returnvalue))
  (`/Engine/EditorBlueprintResources/StandardMacros.IsValid` _output
    (:`Is Valid`
      (`Actor.K2_DestroyActor` _output)
      (`KismetArrayLibrary.Array_Remove` (`self.All_Unit`) _returnvalue)
      (`KismetSystemLibrary.PrintString` "Removed")
      (`self.RealignSquad`))
    (:`Is Not Valid`
      (`KismetSystemLibrary.PrintString` "Nothing to remove"))))

(fn `RealignSquad`
  (`self.ResizeSquadBox`)
  (`self.RepositionUnitsInRow`)
  (return))

(fn `RepositionUnitsInRow`
  (locals (Y_Start :type "Float (double-precision)"))
  (set `local.Y_Start` (* (* (`self.UnitSpacing`) (`KismetArrayLibrary.Array_LastIndex` (`self.All_Unit`))) 0.5 -1.0))
  (for (_array_element _array_index) (`self.All_Unit`)
    (`SceneComponent.K2_SetRelativeLocation` (`Actor.RootComponent` _array_element) (`KismetMathLibrary.MakeVector` 0.0 (+ (* _array_index (`self.UnitSpacing`)) (`local.Y_Start`))) false false)))

(fn `ResizeSquadBox`
  (`BoxComponent.SetBoxExtent` (`self.Squad Box`) (`KismetMathLibrary.MakeVector` 32.0 (* (`KismetArrayLibrary.Array_Length` (`self.All_Unit`)) (/ (`self.UnitSpacing`) 2.0)) 32.0) true)
  (return))