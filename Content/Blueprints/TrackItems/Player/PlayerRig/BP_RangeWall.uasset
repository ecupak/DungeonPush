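; BP_RangeWall is a player rig wall whose Box component is repositioned along world X to match a given range.
; The construction script caches the Box's starting world X as BaseRange.
; SetRange moves the Box to BaseRange minus Range, keeping its Y and Z unchanged.
; The Shot event is an empty stub.
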(event `SetRange`
  (params (Range :type Integer))
  (bind (_returnvalue_x _returnvalue_y _returnvalue_z) (`KismetMathLibrary.BreakVector` (`SceneComponent.K2_GetComponentLocation` (`self.Box`))))
  (`SceneComponent.K2_SetWorldLocation` (`self.Box`) (`KismetMathLibrary.MakeVector` (- (`self.BaseRange`) Range) _returnvalue_y _returnvalue_z) false false))

(event `/Game/Blueprints/Bullet/BPI_Shootable.ReceiveShot`
  (params (Damage :type "Float (double-precision)")))

(fn `UserConstructionScript`
  (bind _returnvalue_x (`KismetMathLibrary.BreakVector` (`SceneComponent.K2_GetComponentLocation` (`self.Box`))))
  (set `self.BaseRange` _returnvalue_x))