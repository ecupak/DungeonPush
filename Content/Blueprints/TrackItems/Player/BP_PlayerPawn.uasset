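; Player pawn for a track runner: auto-moves forward, strafes on input and carries a squad managed by ACSquad.
; StartLevel builds the squad, spawns a camera rig and HUD, places the pawn on the track and enables Tick, where the rig follows only X and Z.
; Damage updates HUD health; fire range changes update HUD and BulletWall.
; Debug keys add or remove units; bullet-spawning logic is left unwired.
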(event Custom|StartLevel
  (Development|PrintString "Pawn starting level")
  (CallFunction|Initialize)
  (Actor|Tick|SetActorTickEnabled true))

(event Game|Damage|EventAnyDamage
  (params (Damage :type Float%20%28single-precision%29) (DamageType :type Damage%20Type%20Object%20Reference) (InstigatedBy :type Controller%20Object%20Reference) (DamageCauser :type Actor%20Object%20Reference))
  (bind _output_get (Variables|Default|SetHP (Math|Float|Max(Float) (- (Variables|Default|GetHP) Damage) 0.0)))
  (Default|SetHealth (Variables|Default|GetHUD_Widget) (/ _output_get (Variables|Default|GetMaxHP))))

(event EventTick
  (params (DeltaSeconds :type Float%20%28single-precision%29))
  (bind _returnvalue (Transformation|GetActorLocation))
  (Pawn|Input|AddMovementInput (* (Transformation|GetActorForwardVector) 0.5) 1.0 false)
  (Transformation|SetActorLocation (Variables|Default|GetRig) (Math|Vector|MakeVector (.x _returnvalue) 0.0 (.z _returnvalue)) false false))

(event EventPossessed
  (params (NewController :type Controller%20Object%20Reference))
  (Input|AddMappingContext (PlayerController|LocalPlayerSubsystems|GetEnhancedInputLocalPlayerSubsystem (.AsPC%20Game (Utilities|Casting|CastToPC_Game NewController))) "/Game/Inputs/IMC_Player.IMC_Player" 0 "(bIgnoreAllPressedKeysUntilRelease=True,bForceImmediately=False,bNotifyUserSettings=False)"))

(event Custom|Bind_OnShootDelayTimer
  (Variables|Default|SetCanShoot true))

(event Input|EnhancedActionEvents|EnhancedInputActionIA_Strafe
  (params (ActionValue :type Float%20%28double-precision%29) (ElapsedSeconds :type Float%20%28double-precision%29) (TriggeredSeconds :type Float%20%28double-precision%29) (InputAction :type Input%20Action%20Object%20Reference :default "/Game/Inputs/IA_Strafe.IA_Strafe"))
  (Pawn|Input|AddMovementInput (* ActionValue (Transformation|GetActorRightVector)) 1.0 false))

(event Input|EnhancedActionEvents|EnhancedInputActionIA_Shoot
  (params (ActionValue :type Boolean) (ElapsedSeconds :type Float%20%28double-precision%29) (TriggeredSeconds :type Float%20%28double-precision%29) (InputAction :type Input%20Action%20Object%20Reference :default "/Game/Inputs/IA_Shoot.IA_Shoot")))

(event Input|KeyboardEvents|DebugKeyUp
  (params (Key :type Key%20Structure :default "None") (ActionValue :type Input%20Action%20Value%20Structure))
  (:Pressed
    (Default|AddUnit (Variables|Default|GetAC_Squad))
    (Pawn|Input|AddMovementInput "0.000000,1.000000,0.000000" 0.001 false) ; Forces collision check update.\nNeeded because enlarging collision box\nnear wall will let you clip through the wall\nuntil you move (force a collision update).
  ))

(event Input|KeyboardEvents|DebugKeyDown
  (params (Key :type Key%20Structure :default "None") (ActionValue :type Input%20Action%20Value%20Structure))
  (:Pressed
    (Default|RemoveUnit (Variables|Default|GetAC_Squad))))

(event Custom|ChangeFireRange
  (params (Delta :type Integer))
  (Variables|Stats|SetFireRange (Math|Integer|Max(Integer) (+ Delta (Variables|Stats|GetFireRange))))
  (Default|SetRange (Variables|Default|GetHUD_Widget) (Variables|Stats|GetFireRange))
  (Default|SetRange (Variables|Default|GetBulletWall) (* (Variables|Stats|GetFireRange) (Variables|Default|GetFireRangeWorldScale))))

(event Custom|SetFireRange
  (Default|SetRange (Variables|Default|GetHUD_Widget) (Variables|Stats|GetFireRange))
  (Default|SetRange (Variables|Default|GetBulletWall) (* (Variables|Stats|GetFireRange) (Variables|Default|GetFireRangeWorldScale))))

(fn ConstructionScript)

(fn GetHeight
  (return (* (.z (Components|Box|GetScaledBoxExtent (Variables|Default|GetSquadBox))) 2.0)))

(fn GetBulletSpawnLocation
  (return (+ (* (Transformation|GetActorForwardVector) (LocalVariables|GetBulletForwardSpawnOffset)) (.location (Transformation|GetActorTransform)))))

(fn AddWidget
  (bind _returnvalue (UserInterface|CreateWidget "/Game/Widgets/WBP_HUD.WBP_HUD_C"))
  (bind _output_get (Variables|Default|SetHUD_Widget _returnvalue))
  (UserInterface|Viewport|AddtoViewport _output_get 0)
  (return))

(fn AddRig
  (bind _returnvalue (Game|SpawnActorfromClass "/Game/Blueprints/TrackItems/Player/PlayerRig/BP_PlayerRig.BP_PlayerRig_C" (Transformation|GetActorTransform) "Undefined" "MultiplyWithRoot" 0 0))
  (bind _output_get (Variables|Default|SetRig _returnvalue))
  (Game|Player|SetViewTargetwithBlend (.AsPC%20Game (Utilities|Casting|CastToPC_Game (Pawn|GetController))) _output_get 0.0 "VTBlend_Linear" 0.0 false)
  (return))

(fn PlaceonTrack
  (Default|PlaceonTrack (Variables|Default|GetAC_PlaceOnTrack) self (CallFunction|GetHeight))
  (return))

(fn Initialize
  (Utilities|FlowControl|Sequence
    (:then_0
      (CallFunction|SetupSquad))
    (:then_1
      (CallFunction|AddRig))
    (:then_2
      (CallFunction|AddWidget))
    (:then_3
      (CallFunction|PlaceonTrack))
    (:then_4
      (return))))

(fn SetupSquad
  (Default|Initialize (Variables|Default|GetAC_Squad) (Variables|Default|GetSquadBox))
  (return))