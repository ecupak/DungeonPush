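; BP_EnemySpawner is a track-item actor that periodically spawns BP_Enemy and makes later enemies tougher over time.
; BeginPlay caches the BP_PlayerPawn and starts looping timers for spawning and difficulty increases.
; Enemies spawn just above the actor at a random Y within its Box extent, initialized with health, player pawn and speed.
; Each difficulty increase increments the health given to new enemies and prints it.
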(event `self.ReceiveBeginPlay`
  (`|ExecutionSequence`
    (:`then_0`
      (bind _returnvalue (`GameplayStatics.GetActorOfClass` "/Game/Blueprints/TrackItems/Player/BP_PlayerPawn.BP_PlayerPawn_C"))
      (set `self.PlayerPawn` _returnvalue))
    (:`then_1`
      (`KismetSystemLibrary.K2_SetTimerDelegate` (`|CreateDelegate` :!event `SpawnEnemy`) (`self.SpawnDelay`) true)
      (`KismetSystemLibrary.K2_SetTimerDelegate` (`|CreateDelegate` :!event `IncreaseDifficulty`) (`self.DifficultyDelay`) true))))

(event `SpawnEnemy`
  (bind _spawnlocation (`self.GetSpawnLocation`))
  (bind _returnvalue (`|SpawnActorFromClass` "/Game/Blueprints/TrackItems/Enemies/BP_Enemy.BP_Enemy_C" (`KismetMathLibrary.MakeTransform` _spawnlocation (`self.K2_GetActorRotation`)) "AlwaysSpawn" "MultiplyWithRoot" null null))
  (`/Game/Blueprints/TrackItems/Enemies/BP_Enemy.Initialize` _returnvalue (`self.EnemyHealth`) (`self.PlayerPawn`) (`self.MovementSpeed`)))

(event `IncreaseDifficulty`
  (bind _result (`/Engine/EditorBlueprintResources/StandardMacros.IncrementFloat` (`self.EnemyHealth`))
    (:`  `
      (`KismetSystemLibrary.PrintText` (`|FormatText` "Enemy HP increased to {x}" _result)))))

(fn `GetSpawnLocation`
  (returns (SpawnLocation :type "Vector Structure"))
  (bind (_returnvalue_x _returnvalue_y _returnvalue_z) (`KismetMathLibrary.BreakVector` (`self.K2_GetActorLocation`)))
  (bind (_returnvalue_x_2 _returnvalue_y_2) (`KismetMathLibrary.BreakVector` (`BoxComponent.GetScaledBoxExtent` (`self.Box`))))
  (return (`KismetMathLibrary.MakeVector` _returnvalue_x (+ (* _returnvalue_y_2 (`KismetMathLibrary.RandomFloatInRange` -1.0 1.0)) _returnvalue_y) (+ _returnvalue_z 20.0))))

(fn `UserConstructionScript`)