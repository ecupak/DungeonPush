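; Enemy for track gameplay that either moves toward the end or chases the player, switched by a chase-mode event.
; Initialize supplies health, player pawn and speed, and derives attack power as half its health.
; Shot lowers health and updates a health bar widget, destroying the enemy only when health equals exactly zero.
; Overlapping the player pawn applies damage, destroys the enemy and prints the amount.
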(event `self.ReceiveBeginPlay`
  (`parent.ReceiveBeginPlay`)
  (bind _aswbp_health_bar (cast `/Game/Widgets/WBP_HealthBar` (`WidgetComponent.GetWidget` (`self.HPBar`))))
  (set `self.HP_BarWidget` _aswbp_health_bar))

(event `/Game/Blueprints/Bullet/BPI_Shootable.ReceiveShot`
  (params (Damage :type "Float (double-precision)"))
  (bind _output_get (set `self.HP` (- (`self.HP`) Damage)))
  (if (== _output_get 0.0)
    (`self.K2_DestroyActor`)
    (else
      (`/Game/Widgets/WBP_HealthBar.SetPercent` (`self.HP_BarWidget`) (/ (`self.HP`) (`self.MaxHP`))))))

(event `self.ReceiveTick`
  (params (DeltaSeconds :type "Float (single-precision)"))
  (switch `/Game/Blueprints/TrackItems/Enemies/EMoveMode` (`self.MovementMode`)
    (:`NewEnumerator0`
      (`self.MoveTowardsEnd`))
    (:`NewEnumerator1`
      (`self.ChasePlayer`))))

(event `ActivateChaseMode`
  (set `self.MovementMode` "NewEnumerator1"))

(event `self.ReceiveActorBeginOverlap`
  (params (OtherActor :type "Actor Object Reference"))
  (bind _attackpower (`self.AttackPower`))
  (bind _asbp_player_pawn (cast `/Game/Blueprints/TrackItems/Player/BP_PlayerPawn` OtherActor))
  (`GameplayStatics.ApplyDamage` _asbp_player_pawn _attackpower)
  (`self.K2_DestroyActor`)
  (`KismetSystemLibrary.PrintText` (`|FormatText` "Did {x} damage" _attackpower) true true (struct :`R` 1.0 :`G` 0.028286 :`A` 1.0)))

(fn `ChasePlayer`
  (`self.AddMovementInput` (* (`self.MovementSpeed`) (`self.GetVectorTowardsPlayer` true)))
  (return))

(fn `GetHeight`
  (returns (Height :type "Float (double-precision)"))
  (bind (_returnvalue_x _returnvalue_y _returnvalue_z) (`KismetMathLibrary.BreakVector` (`SceneComponent.K2_GetComponentScale` (`self.Cylinder`))))
  (return (* _returnvalue_z 100.0)))

(fn `GetVectorTowardsPlayer`
  (params (Normalized :type Boolean :default true))
  (returns (VectorToPlayer :type "Vector Structure"))
  (bind _returnvalue (- (`SceneComponent.K2_GetComponentLocation` (`Actor.RootComponent` (`self.PlayerPawn`))) (`SceneComponent.K2_GetComponentLocation` (`self.Box`))))
  (return (`KismetMathLibrary.SelectVector` (`KismetMathLibrary.Normal` _returnvalue) _returnvalue Normalized)))

(fn `Initialize`
  (params (InitHP :type "Float (double-precision)") (InitPawn :type "/Game/Blueprints/TrackItems/Player/BP_PlayerPawn Object Reference") (InitSpeed :type "Float (double-precision)"))
  (`|ExecutionSequence`
    (:`then_0`
      (bind _output_get (set `self.MaxHP` (`local.InitHP`)))
      (bind _output_get_2 (set `self.HP` _output_get))
      (set `self.AttackPower` (/ _output_get_2 2.0)))
    (:`then_1`
      (set `self.PlayerPawn` (`local.InitPawn`)))
    (:`then_2`
      (set `self.MovementSpeed` (`local.InitSpeed`)))))

(fn `UserConstructionScript`)